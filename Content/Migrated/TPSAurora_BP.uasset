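; TPSAurora_BP is a character Blueprint, apparently third-person, that handles turn-in-place detection on the Turn input axis.
; It sets TurnRight or TurnLeft when control yaw leads actor yaw by over 90 degrees either way, clearing both only at exactly zero.
; All three cases enable both controller-desired rotation and orient-to-movement on CharacterMovement.
; AddControllerYawInput receives a constant zero rather than the axis value.
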(event EventBeginPlay)

(event Collision|EventActorBeginOverlap
  (params (OtherActor :type Actor%20Object%20Reference)))

(event EventTick
  (params (DeltaSeconds :type Float%20%28single-precision%29)))

(event Input|AxisEvents|InputAxisTurn
  (params (AxisValue :type Float%20%28single-precision%29))
  (bind _returnvalue (Pawn|GetControlRotation :!class /Script/Engine.Pawn))
  (bind _returnvalue_2 (Transformation|GetActorRotation))
  (bind _charactermovement (Variables|Character|GetCharacterMovement))
  (bind _charactermovement_2 (Variables|Character|GetCharacterMovement))
  (bind _charactermovement_3 (Variables|Character|GetCharacterMovement))
  (bind _returnvalue_3 (Math|Rotator|Delta(Rotator) _returnvalue _returnvalue_2))
  (Pawn|Input|AddControllerYawInput 0.0)
  (Utilities|FlowControl|Sequence
    (:then_0
      (if (> (.yaw _returnvalue_3) 9e+01)
        (Variables|Default|SetTurnRight? true)
        (Variables|/Script/Engine.CharacterMovementComponent|SetbUseControllerDesiredRotation _charactermovement true)
        (Variables|/Script/Engine.CharacterMovementComponent|SetbOrientRotationToMovement _charactermovement_2 true)))
    (:then_1
      (if (< (.yaw _returnvalue_3) -9e+01)
        (Variables|Default|SetTurnLeft? true)
        (Variables|/Script/Engine.CharacterMovementComponent|SetbUseControllerDesiredRotation _charactermovement true)
        (Variables|/Script/Engine.CharacterMovementComponent|SetbOrientRotationToMovement _charactermovement_2 true)))
    (:then_2
      (if (== (.yaw _returnvalue_3) 0.0)
        (Variables|/Script/Engine.CharacterMovementComponent|SetbUseControllerDesiredRotation _charactermovement_3 true)
        (Variables|/Script/Engine.CharacterMovementComponent|SetbOrientRotationToMovement _charactermovement_3 true)
        (Variables|Default|SetTurnRight? false)
        (Variables|Default|SetTurnLeft? false)))))

(fn ConstructionScript)